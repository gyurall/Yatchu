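; Test Blueprint in the Yatchu game that experiments with updating a text render from a replication callback.
; The RepNotify for NewVar_0 calls ReqNum, which sets the text to a fixed number, and ResNum forwards to the same event.
; Disconnected leftovers bind an empty custom event to the HUD dice widget's roll click, set its Aces number, print a string and call ResNum.
; Tick and the construction script are empty.
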(event Custom|ReqNum
  (Rendering|Components|TextRender|SetText (Variables|Default|GetTextRender) (Utilities|Text|ToText(Integer) 1)))

(event Custom|커스텀이벤트_0)

(event Custom|ResNum
  (CallFunction|ReqNum))

(event EventTick
  (params (DeltaSeconds :type Float%20%28single-precision%29)))

(fn ConstructionScript)

(fn OnRepNewVar0
  (CallFunction|ReqNum))