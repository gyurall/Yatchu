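; BP_Round is an actor that displays the current round number of the Yatchu game through a text render component.
; On every Tick it casts the player's HUD to YatchuHud and binds an event for round number changes, repeating the bind each frame.
; BPRoundAutoGenFunc increments a counter, converts it to text, and writes it to the Round variable and text render of the BP_Round found by GetActorOfClass.
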(event Collision|EventActorBeginOverlap
  (params (OtherActor :type Actor%20Object%20Reference)))

(event EventTick
  (params (DeltaSeconds :type Float%20%28single-precision%29))
  (bind _asyatchu_hud (Utilities|Casting|CastToYatchuHud (HUD|GetHUD (Game|GetPlayerController 0))))
  (EventDispatchers|BindEventtoChangeRoundNumber _asyatchu_hud (EventDispatchers|CreateEvent :!event BPRoundAutoGenFunc)))

(fn ConstructionScript)

(fn BPRoundAutoGenFunc
  (bind _returnvalue (Actor|GetActorOfClass "BP_Round_C"))
  (bind _output_get (Variables|Default|SetNewVar_0 (+ (Variables|Default|GetNewVar_0) 1)))
  (bind _output_get_2 (Variables|BP_Round_C|SetRound _returnvalue (Utilities|Text|ToText(Integer) _output_get)))
  (Rendering|Components|TextRender|SetText (Variables|BP_Round_C|GetTextRender _returnvalue) _output_get_2))