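; BP_Aces is a Yatchu dice game actor that displays the Aces number in world text after a roll click.
; On every Tick it casts the first player's HUD to YatchuHud and binds a custom event to the DiceWidget's roll click again.
; That event calls ResNum, which gets the value from the widget's SetAcesNum and passes it to ReqNum to write into the TextRender.
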(event Custom|ReqNum
  (params (NewParam :type Integer))
  (Rendering|Components|TextRender|SetText (Variables|Default|GetTextRender) (Utilities|Text|ToText(Integer) NewParam)))

(event Custom|ResNum
  (bind _newparam (Default|SetAcesNum (Variables|/Game/Yatchu/Games/Main/YatchuHud.YatchuHud_C|GetDiceWidget (stale EventTick _asyatchu_hud))))
  (CallFunction|ReqNum _newparam))

(event Custom|커스텀이벤트_0
  (CallFunction|ResNum))

(event EventTick
  (params (DeltaSeconds :type Float%20%28single-precision%29))
  (bind _asyatchu_hud (Utilities|Casting|CastToYatchuHud (HUD|GetHUD (Game|GetPlayerController 0))))
  (EventDispatchers|BindEventtoClickRoll (Variables|/Game/Yatchu/Games/Main/YatchuHud.YatchuHud_C|GetDiceWidget _asyatchu_hud) (delegate Custom|커스텀이벤트_0)))

(fn ConstructionScript)