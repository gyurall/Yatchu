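; BP_ThreeOfAKind shows the Three of a Kind score of the Yatchu dice game on a text render component.
; Every Tick it gets the YatchuHud from player controller 0 and binds a custom event to the dice widget's roll click.
; On a roll, ResNum fetches the value from the widget's SetThreeOfAKindNum and ReqNum writes it to the text.
; An auto-generated Aces-named function only prints a debug string.
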(event Custom|커스텀이벤트_1
  (CallFunction|ResNum))

(event Custom|ReqNum
  (params (NewParam :type Integer))
  (Rendering|Components|TextRender|SetText (Variables|Default|GetTextRender) (Utilities|Text|ToText(Integer) NewParam)))

(event Custom|ResNum
  (bind _newparam (Default|SetThreeOfAKindNum (Variables|/Game/Yatchu/Games/Main/YatchuHud.YatchuHud_C|GetDiceWidget (stale EventTick _asyatchu_hud))))
  (CallFunction|ReqNum _newparam))

(event EventTick
  (params (DeltaSeconds :type Float%20%28single-precision%29))
  (bind _asyatchu_hud (Utilities|Casting|CastToYatchuHud (HUD|GetHUD (Game|GetPlayerController 0))))
  (EventDispatchers|BindEventtoClickRoll (Variables|/Game/Yatchu/Games/Main/YatchuHud.YatchuHud_C|GetDiceWidget _asyatchu_hud) (delegate Custom|커스텀이벤트_1)))

(fn ConstructionScript)

(fn BPAcesAutoGenFunc
  (Development|PrintString "Hello"))